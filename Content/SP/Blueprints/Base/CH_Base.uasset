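; CH_Base is a base Character Blueprint for gamepad-driven movement, facing, interaction and multi-level crouching.
; The left stick moves relative to control yaw, while right-stick input interpolates actor rotation and suspends orient-to-movement.
; The interact action calls StartInteractionMessage on the stored Interagivel, cast to A_Base or CH_Enemy_Base.
; The crouch action cycles LevelCrouch through Abaixar and Levantar, adjusting capsule radius and scaling crouched speed by level.
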(event Input|ActionEvents|InputActionActionToInteract
  (params (Key :type Key%20Structure :default "None"))
  (bind _interagivel (Variables|Default|Getinteragivel))
  ;[1 1 1] Interação com Actors
  (:Pressed
    (if (!= (Variables|Default|Getinteragivel) 0)
      (bind _asa_base (Utilities|Casting|CastToA_Base _interagivel)
        (:then
          (Class|InterfaceInteraction|StartInteraction(Message) _asa_base))
        (:CastFailed
          (bind _asch_enemy_base (Utilities|Casting|CastToCH_Enemy_Base _interagivel))
          (Class|InterfaceInteraction|StartInteraction(Message) _asch_enemy_base))))))

(event Input|ActionEvents|InputActionActionToCrouch
  (params (Key :type Key%20Structure :default "None"))
  ;[1 1 1] Agaixando
  (:Pressed
    (if true
      (Development|PrintString "Hello")
      (bind _result (Math|Integer|IncrementInt (Variables|AboutCrouch|GetlevelCrouch))
        (:%20%20
          (if (> _result 2)
            (bind _output_get (Variables|AboutCrouch|SetlevelCrouch 0)))
          (switch int _output_get
            (:Default
              (CallFunction|Abaixar :!label _label)
              (Development|PrintString "Abaixar"))
            (:0
              (CallFunction|Levantar)
              (Development|PrintString "Levantar"))
            (:1
              (goto _label))))))))

(event Input|AxisEvents|InputAxisAnalogicRightX
  (params (AxisValue :type Float%20%28single-precision%29))
  (bind _returnvalue (Transformation|GetActorRotation))
  (bind (_roll _pitch) (Math|Rotator|BreakRotator _returnvalue))
  ;[1 1 1] Analogico Direito
  (bind _output_get (Variables|Default|SetusingAnalogicRight (or (!= AxisValue 0.0) (!= (stale Input|AxisEvents|InputAxisAnalogicRightY AxisValue) 0.0))))
  (if _output_get
    (Variables|/Script/Engine.CharacterMovementComponent|SetbOrientRotationToMovement (Variables|Character|GetCharacterMovement) false)
    (Transformation|SetActorRotation (Math|Interpolation|RInterpTo _returnvalue (Math|Rotator|MakeRotator _roll _pitch (Class|KismetMathLibrary|DegAtan2 AxisValue (stale Input|AxisEvents|InputAxisAnalogicRightY AxisValue))) (Utilities|Time|GetWorldDeltaSeconds) (Variables|Default|GetspeedOfRotation)))
    (else
      (Variables|/Script/Engine.CharacterMovementComponent|SetbOrientRotationToMovement (Variables|Character|GetCharacterMovement) true))))

(event Input|AxisEvents|InputAxisAnalogicRightY
  (params (AxisValue :type Float%20%28single-precision%29))
  (bind _returnvalue (Transformation|GetActorRotation))
  (bind (_roll _pitch) (Math|Rotator|BreakRotator _returnvalue))
  ;[1 1 1] Analogico Direito
  (bind _output_get (Variables|Default|SetusingAnalogicRight (or (!= (stale Input|AxisEvents|InputAxisAnalogicRightX AxisValue) 0.0) (!= AxisValue 0.0))))
  (if _output_get
    (Variables|/Script/Engine.CharacterMovementComponent|SetbOrientRotationToMovement (Variables|Character|GetCharacterMovement) false)
    (Transformation|SetActorRotation (Math|Interpolation|RInterpTo _returnvalue (Math|Rotator|MakeRotator _roll _pitch (Class|KismetMathLibrary|DegAtan2 (stale Input|AxisEvents|InputAxisAnalogicRightX AxisValue) AxisValue)) (Utilities|Time|GetWorldDeltaSeconds) (Variables|Default|GetspeedOfRotation)))
    (else
      (Variables|/Script/Engine.CharacterMovementComponent|SetbOrientRotationToMovement (Variables|Character|GetCharacterMovement) true))))

(event Input|AxisEvents|InputAxisAnalogicLeftX
  (params (AxisValue :type Float%20%28single-precision%29))
  ;[1 1 1] Analogico Esquerdo
  (Pawn|Input|AddMovementInput (Math|Vector|GetRightVector (Math|Rotator|MakeRotator 0.0 0.0 (.Yaw (Math|Rotator|BreakRotator (Pawn|GetControlRotation :!class /Script/Engine.Pawn))))) AxisValue false))

(event Input|AxisEvents|InputAxisAnalogicLeftY
  (params (AxisValue :type Float%20%28single-precision%29))
  ;[1 1 1] Analogico Esquerdo
  (Variables|Default|SetusingAnalogicLeft (or (!= AxisValue 0.0) (!= (stale Input|AxisEvents|InputAxisAnalogicLeftX AxisValue) 0.0)))
  (Pawn|Input|AddMovementInput (Math|Vector|GetForwardVector (Math|Rotator|MakeRotator 0.0 0.0 (.Yaw (Math|Rotator|BreakRotator (Pawn|GetControlRotation :!class /Script/Engine.Pawn))))) AxisValue false))

(fn ConstructionScript)

(fn Abaixar
  (Variables|/Script/Engine.CharacterMovementComponent|SetMaxWalkSpeedCrouched (Variables|Character|GetCharacterMovement) (/ (Class|MovementComponent|GetMaxSpeed (Variables|Character|GetCharacterMovement)) (Math|Conversions|ToFloat(Integer) (+ (Variables|AboutCrouch|GetlevelCrouch) 1))))
  (Components|Capsule|SetCapsuleRadius (Variables|Collision|GetCapsuleComponent) 2e+01 true)
  (Character|Crouch))

(fn Levantar
  (Components|Capsule|SetCapsuleRadius (Variables|Collision|GetCapsuleComponent) 42.0 true)
  (Character|UnCrouch))