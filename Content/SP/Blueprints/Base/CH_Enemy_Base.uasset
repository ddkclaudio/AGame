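; CH_Enemy_Base is a base enemy Blueprint that registers itself as an interactable for CH_Base characters.
; A Box overlap sets the other character's Interagivel reference to this enemy, and leaving clears it without checking which object it holds.
; StartInteraction only prints a debug message, as placeholder behavior alongside the ON and OFF overlap prints.
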(event OnComponentBeginOverlap(Box)
  (params (OverlappedComponent :type Primitive%20Component%20Object%20Reference) (OtherActor :type Actor%20Object%20Reference) (OtherComp :type Primitive%20Component%20Object%20Reference) (OtherBodyIndex :type Integer) (bFromSweep :type Boolean) (SweepResult :type Hit%20Result%20Structure%20%28by%20ref%29))
  ;[1 1 1] Comment
  (if (!= OtherActor self)
    (bind _asch_base (Utilities|Casting|CastToCH_Base OtherActor))
    (Variables|/Game/SP/Blueprints/Base/CH_Base.CH_Base_C|Setinteragivel _asch_base self)
    (Development|PrintString "CH_Enemy_Base: ON")))

(event OnComponentEndOverlap(Box)
  (params (OverlappedComponent :type Primitive%20Component%20Object%20Reference) (OtherActor :type Actor%20Object%20Reference) (OtherComp :type Primitive%20Component%20Object%20Reference) (OtherBodyIndex :type Integer))
  ;[1 1 1] Comment
  (bind _asch_base (Utilities|Casting|CastToCH_Base OtherActor))
  (Variables|/Game/SP/Blueprints/Base/CH_Base.CH_Base_C|Setinteragivel _asch_base 0)
  (Development|PrintString "CH_Enemy_Base: OFF"))

(event EventStartInteraction
  (Development|PrintString "CH_Enemy_Base: Action" true true "(R=0.101204,G=1.000000,B=0.134408,A=1.000000)"))

(fn ConstructionScript
  (|CallParentFunction))